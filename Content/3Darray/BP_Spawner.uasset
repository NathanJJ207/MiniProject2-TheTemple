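; BP_Spawner fills a 3D grid with instances of an Actor class at BeginPlay, starting from its root's world location.
; It resizes the NZ array to Z and loops over it for the layers, with a flattened X×Y loop inside.
; Division and modulo by Y give each cell's position, scaled by per-axis spacing.
; Spawns are scaled down, and each location overwrites ActorLocation.
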(event EventBeginPlay
  (bind _nz (Variables|Default|GetNZ))
  (bind _y (Variables|Default|GetY))
  ;[1 1 1] 3D
  (Utilities|Array|Resize _nz (Variables|Default|GetZ))
  (for (_ _array_index) _nz
    ;[1 1 1] 2D
    (for _index (range 0 (- (* (Variables|Default|GetX) (Variables|Default|GetY)) 1))
      (bind _returnvalue (Game|SpawnActorfromClass (Variables|Default|GetActor) (Math|Transform|MakeTransform (+ (Transformation|GetWorldLocation (Variables|Default|GetDefaultSceneRoot)) (Math|Vector|MakeVector (* (/ _index _y) (Variables|Default|GetSpaceX)) (* (Math|Integer|%(Integer) _index _y) (Variables|Default|GetSpaceY)) (* _array_index (Variables|Default|GetSpaceZ)))) "0, 0, 0" "0.100000,0.100000,0.100000") "Undefined" 0 0))
      (Variables|Default|SetActorLocation (Transformation|GetWorldLocation (Variables|/Script/Engine.Actor|GetRootComponent _returnvalue))))))

(fn ConstructionScript)